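; BP_Barrier2 is a moving barrier that slides back and forth endlessly along the world X axis.
; On BeginPlay it stores its start location, then a Timeline lerps X toward a fixed offset in the negative direction, keeping Y and Z unchanged.
; When the Timeline finishes, its direction selects MoveToStart or MoveToEnd, creating a continuous ping-pong loop.
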(event Custom|Move%20to%20start
  (bind _locztion (Variables|Default|GetLocztion))
  (bind (_direction _alpha) (Timeline|Timeline ReverseFromEnd)
    (:Update
      (Transformation|SetActorLocation (Math|Vector|MakeVector (Math|Float|Lerp (.x _locztion) (- (.x _locztion) 4.2e+02) _alpha) (.y _locztion) (.z _locztion)) false false))
    (:Finished
      (switch Utilities|FlowControl|Switch|SwitchonETimelineDirection _direction
        (:Forward
          (CallFunction|MovetoStart))
        (:Backward
          (CallFunction|MovetoEnd))))))

(event Custom|Move%20to%20end
  (bind _locztion (Variables|Default|GetLocztion))
  (bind (_direction _alpha) (Timeline|Timeline PlayFromStart)
    (:Update
      (Transformation|SetActorLocation (Math|Vector|MakeVector (Math|Float|Lerp (.x _locztion) (- (.x _locztion) 4.2e+02) _alpha) (.y _locztion) (.z _locztion)) false false))
    (:Finished
      (switch Utilities|FlowControl|Switch|SwitchonETimelineDirection _direction
        (:Forward
          (CallFunction|MovetoStart))
        (:Backward
          (CallFunction|MovetoEnd))))))

(event EventBeginPlay
  (Variables|Default|SetLocztion (Transformation|GetActorLocation))
  (CallFunction|MovetoEnd))

(fn ConstructionScript)