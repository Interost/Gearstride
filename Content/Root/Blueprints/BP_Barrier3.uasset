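; BP_Barrier3 is a barrier actor that slides back and forth along the world Y axis without stopping.
; It caches its location on BeginPlay, and a Timeline lerps Y between that origin and a fixed offset while X and Z stay at the cached values.
; When the Timeline finishes, its direction selects the move-to-start or move-to-end event, creating an endless ping-pong loop.
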(event Custom|Move%20to%20start
  (bind _locztion (Variables|Default|GetLocztion))
  (bind (_direction _alpha) (Timeline|Timeline ReverseFromEnd)
    (:Update
      (Transformation|SetActorLocation (Math|Vector|MakeVector (.x _locztion) (Math|Float|Lerp (.y _locztion) (+ (.y _locztion) 3.1e+02) _alpha) (.z _locztion)) false false))
    (:Finished
      (switch Utilities|FlowControl|Switch|SwitchonETimelineDirection _direction
        (:Forward
          (CallFunction|MovetoStart))
        (:Backward
          (CallFunction|MovetoEnd))))))

(event Custom|Move%20to%20end
  (bind _locztion (Variables|Default|GetLocztion))
  (bind (_direction _alpha) (Timeline|Timeline PlayFromStart)
    (:Update
      (Transformation|SetActorLocation (Math|Vector|MakeVector (.x _locztion) (Math|Float|Lerp (.y _locztion) (+ (.y _locztion) 3.1e+02) _alpha) (.z _locztion)) false false))
    (:Finished
      (switch Utilities|FlowControl|Switch|SwitchonETimelineDirection _direction
        (:Forward
          (CallFunction|MovetoStart))
        (:Backward
          (CallFunction|MovetoEnd))))))

(event EventBeginPlay
  (Variables|Default|SetLocztion (Transformation|GetActorLocation))
  (CallFunction|MovetoEnd))

(fn ConstructionScript)