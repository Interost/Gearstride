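; BP_BlueColumn is a column actor that rises when a blue button signals it.
; On BeginPlay it finds all BP_BlueButton actors and binds its Up event to their column-up dispatcher.
; Up stores the current height, then a timeline lerps the actor's Z position 100 units upward from it.
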(event Custom|Up
  (bind _returnvalue (Transformation|GetActorLocation))
  (Variables|Default|SetLocZ (.z (Transformation|GetActorLocation)))
  (bind _alpha (Timeline|Timeline Play)
    (:Update
      (Transformation|SetActorLocation (Math|Vector|MakeVector (.x _returnvalue) (.y _returnvalue) (Math|Float|Lerp (Variables|Default|GetLocZ) (+ (Variables|Default|GetLocZ) 1e+02) _alpha)) false false))))

(event Collision|EventActorBeginOverlap
  (params (OtherActor :type Actor%20Object%20Reference)))

(event EventTick
  (params (DeltaSeconds :type Float%20%28single-precision%29)))

(event EventBeginPlay
  (bind _outactors (Actor|GetAllActorsOfClass "/Game/Root/Blueprints/BP_BlueButton.BP_BlueButton_C"))
  (EventDispatchers|BindEventtoColumnUp _outactors (delegate Custom|Up)))

(fn ConstructionScript)