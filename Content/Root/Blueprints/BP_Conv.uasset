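; BP_Conv is a conveyor-style actor that pushes whatever overlaps it along a set direction.
; Every Tick it gets the actors overlapping its Collision component and adds a world offset to each, with no sweep, so blocking geometry does not stop them.
; The Speed function builds that offset from the Arrow component's forward vector, the Speed variable and delta seconds, so the arrow sets direction and movement is frame-rate independent.
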(event EventTick
  (params (DeltaSeconds :type Float%20%28single-precision%29))
  (|CallParentFunction DeltaSeconds)
  (for _array_element (Collision|GetOverlappingActors (Variables|Default|GetCollision) 0 :!class /Script/Engine.PrimitiveComponent)
    (Transformation|AddActorWorldOffset _array_element (CallFunction|Speed))))

(fn ConstructionScript)

(fn Speed
  (return (* (Math|Vector|GetForwardVector (Transformation|GetWorldRotation (Variables|Default|GetArrow))) (* (LocalVariables|GetSpeed) (Utilities|Time|GetWorldDeltaSeconds)))))