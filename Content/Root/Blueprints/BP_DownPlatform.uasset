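; Platform actor that lowers when a BP_PlatCharacter with a true CharStatus overlaps it.
; The overlap event casts the other actor, then plays a timeline that lerps a component's relative Z down by 400 units.
; A Check guard gates the trigger, but the node that sets it to 1 is never executed.
; GetCharacterStatus is a stub returning false, and the construction script is empty.
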(event Collision|EventActorBeginOverlap
  (params (OtherActor :type Actor%20Object%20Reference))
  (if (not (== (Variables|Default|GetCheck) 1))
    (bind _asbp_plat_character (Utilities|Casting|CastToBP_PlatCharacter OtherActor))
    (if (== (Variables|/Game/Root/Blueprints/Character/BP_PlatCharacter.BP_PlatCharacter_C|GetCharStatus _asbp_plat_character) true)
      (bind _newtrack_0 (Timeline|Timeline Play)
        (:Update
          (Transformation|SetRelativeLocation (Variables|Default|Get%20) (Math|Vector|MakeVector 0.0 0.0 (Math|Float|Lerp 0.0 -4e+02 _newtrack_0)) false false))))))

(fn ConstructionScript)

(fn GetCharacterStatus
  (return false))