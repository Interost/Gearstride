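; BP_RedDoor is a door actor that slides open in response to the red button's event.
; On BeginPlay it finds the BP_redButton actors and binds its Open event to their RedDoorOpen dispatcher.
; Open captures the current Y location, then plays a timeline that lerps the door along world Y by a fixed offset.
; The graph has no closing logic.
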(event Custom|Open
  (bind _returnvalue (Transformation|GetActorLocation))
  (Variables|Default|SetLocY (.y (Transformation|GetActorLocation)))
  (bind _alpha (Timeline|Timeline Play)
    (:Update
      (Transformation|SetActorLocation (Math|Vector|MakeVector (.x _returnvalue) (Math|Float|Lerp (Variables|Default|GetLocY) (+ (Variables|Default|GetLocY) 1.8e+02) _alpha) (.z _returnvalue)) false false))))

(event EventBeginPlay
  (bind _outactors (Actor|GetAllActorsOfClass "/Game/Root/Blueprints/BP_redButton.BP_redButton_C"))
  (EventDispatchers|BindEventtoRedDoorOpen _outactors (delegate Custom|Open)))

(event Collision|EventActorBeginOverlap
  (params (OtherActor :type Actor%20Object%20Reference)))

(event EventTick
  (params (DeltaSeconds :type Float%20%28single-precision%29)))

(fn ConstructionScript)