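; Yellow pressure button that a BP_PlatCharacter triggers by overlapping it while its CharStatus is true.
; A timeline lerps a component's relative Z downward to sink the button, then calls CallYellowDoor on finish, presumably to signal the yellow door.
; The Check guard never latches here, since the timeline only sets it to false.
; GetCharacterStatus is a stub that returns false.
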(event Collision|EventActorBeginOverlap
  (params (OtherActor :type Actor%20Object%20Reference))
  (if (not (== (Variables|Default|GetCheck) true))
    (bind _asbp_plat_character (Utilities|Casting|CastToBP_PlatCharacter OtherActor))
    (if (== (Variables|/Game/Root/Blueprints/Character/BP_PlatCharacter.BP_PlatCharacter_C|GetCharStatus _asbp_plat_character) true)
      (bind _newtrack_0 (Timeline|Timeline Play)
        (:Update
          (Transformation|SetRelativeLocation (Variables|Default|Get%20) (Math|Vector|MakeVector 0.0 0.0 (Math|Float|Lerp 0.0 -17.0 _newtrack_0)) false false)
          (Variables|Default|SetCheck false))
        (:Finished
          (Default|CallYellowDoor))))))

(fn ConstructionScript)

(fn GetCharacterStatus
  (return false))