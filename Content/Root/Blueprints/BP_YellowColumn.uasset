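; BP_YellowColumn is a column actor that rises vertically in response to yellow buttons.
; On BeginPlay it finds all BP_YellowButton actors in the level and binds its Up event to their yellow-door event.
; Up stores the current height, then plays a timeline that lerps the column upward by a fixed offset, keeping X and Y unchanged.
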(event Custom|Up
  (bind _returnvalue (Transformation|GetActorLocation))
  (Variables|Default|SetLocZ (.z (Transformation|GetActorLocation)))
  (bind _alpha (Timeline|Timeline Play)
    (:Update
      (Transformation|SetActorLocation (Math|Vector|MakeVector (.x _returnvalue) (.y _returnvalue) (Math|Float|Lerp (Variables|Default|GetLocZ) (+ (Variables|Default|GetLocZ) 5.9e+02) _alpha)) false false))))

(event EventBeginPlay
  (bind _outactors (Actor|GetAllActorsOfClass "/Game/Root/Blueprints/BP_YellowButton.BP_YellowButton_C"))
  (EventDispatchers|BindEventtoYellowDoor _outactors (delegate Custom|Up)))

(fn ConstructionScript)