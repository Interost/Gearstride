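; BP_YellowDoor is a door actor that slides open when triggered by a BP_YellowButton.
; On BeginPlay it finds all BP_YellowButton actors and binds its Open event to their YellowDoor dispatcher.
; Open captures the current X location and plays a timeline that lerps the actor along world X by a fixed offset, with no closing logic.
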(event Custom|Open
  (bind _returnvalue (Transformation|GetActorLocation))
  (Variables|Default|SetLocX (.x (Transformation|GetActorLocation)))
  (bind _alpha (Timeline|Timeline Play)
    (:Update
      (Transformation|SetActorLocation (Math|Vector|MakeVector (Math|Float|Lerp (Variables|Default|GetLocX) (+ (Variables|Default|GetLocX) 1.9e+02) _alpha) (.y _returnvalue) (.z _returnvalue)) false false))))

(event EventBeginPlay
  (bind _outactors (Actor|GetAllActorsOfClass "/Game/Root/Blueprints/BP_YellowButton.BP_YellowButton_C"))
  (EventDispatchers|BindEventtoYellowDoor _outactors (delegate Custom|Open)))

(event Collision|EventActorBeginOverlap
  (params (OtherActor :type Actor%20Object%20Reference)))

(event EventTick
  (params (DeltaSeconds :type Float%20%28single-precision%29)))

(fn ConstructionScript)